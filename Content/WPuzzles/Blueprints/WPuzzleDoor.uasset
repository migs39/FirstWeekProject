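; WPuzzleDoor is a door Blueprint that opens a puzzle UI when clicked.
; ClickedBy defers to the parent implementation, and if that returns true, adds a widget of the Puzzle class to player 0's viewport.
; It passes itself as the Door reference to both that widget and the PuzzlePawn, cast to WPuzzlePawn.
; The construction script only calls its parent, and NewFunction is an empty stub.
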(fn ConstructionScript
  (|CallParentFunction))

(fn Clickedby
  (params (Clicker :type Pawn%20Object%20Reference))
  (bind _returnvalue (UserInterface|CreateWidget (Variables|Default|GetPuzzle) (Game|GetPlayerController 0)))
  (bind _possessed (|CallParentFunction Clicker))
  (if _possessed
    (bind _output_get (Variables|Default|SetWidget _returnvalue))
    (UserInterface|Viewport|AddtoViewport _output_get 0)
    (Variables|/Game/WPuzzles/Blueprints/BasicPuzzleWidget.BasicPuzzleWidget_C|Setdoor (Variables|Default|GetWidget) self)
    (bind _aswpuzzle_pawn (Utilities|Casting|CastToWPuzzlePawn (Variables|Default|GetPuzzlePawn)))
    (Variables|/Game/WPuzzles/Blueprints/WPuzzlePawn.WPuzzlePawn_C|SetDoor _aswpuzzle_pawn self)))

(fn NewFunction)