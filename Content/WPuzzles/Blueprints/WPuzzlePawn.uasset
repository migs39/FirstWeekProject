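; WPuzzlePawn is a pawn that the player temporarily possesses during a puzzle, apparently one tied to a door.
; Its PossessesBy override teleports it to the current player pawn's location and rotation, then calls the parent implementation.
; The cancel input calls Unpossesess, which hides the mouse cursor, has the player controller possess InPawn again and removes the Door's widget from screen.
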(event Input|EnhancedActionEvents|EnhancedInputActionIA_Cancel
  (params (ActionValue :type Boolean) (ElapsedSeconds :type Float%20%28double-precision%29) (TriggeredSeconds :type Float%20%28double-precision%29) (InputAction :type Input%20Action%20Object%20Reference :default "/Game/FirstPerson/Input/Actions/IA_Cancel.IA_Cancel"))
  (:Started
    (CallFunction|Unpossesess)))

(event EventUnpossesess
  (bind _returnvalue (Game|GetPlayerController 0))
  (Variables|/Script/Engine.PlayerController|SetbShowMouseCursor _returnvalue false)
  (Pawn|Possess _returnvalue (Variables|Default|GetInPawn))
  (Widget|RemovefromParent (Variables|/Game/WPuzzles/Blueprints/WPuzzleDoor.WPuzzleDoor_C|GetWidget (Variables|Default|GetDoor))))

(fn ConstructionScript
  (|CallParentFunction))

(fn Possessesby
  (params (pawnIn :type Pawn%20Object%20Reference))
  (bind _returnvalue (Game|Player|GetPlayerPawn 0))
  (Transformation|SetActorRotation self (Transformation|GetActorRotation _returnvalue) true)
  (Transformation|SetActorLocation self (Transformation|GetActorLocation _returnvalue) false true)
  (|CallParentFunction pawnIn))