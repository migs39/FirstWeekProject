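; BP_BackBall is a clickable puzzle sphere that lets the player back out of puzzle control and also shows when the puzzle is solved.
; Clicking it casts the player pawn to BP_PuzzlePawn and calls its unpossess function, printing a debug message if the cast fails.
; A Finished event, triggered from outside, sets IsDone, swaps the sphere to the done material and opens the linked PuzzleDoor.
; The construction script applies that material when IsDone is already set.
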(event OnClicked(Sphere)
  (params (TouchedComponent :type Primitive%20Component%20Object%20Reference) (ButtonPressed :type Key%20Structure :default "None"))
  (bind _asbp_puzzle_pawn (Utilities|Casting|CastToBP_PuzzlePawn (Game|Player|GetPlayerPawn 0))
    (:then
      (Default|Unpossesess _asbp_puzzle_pawn))
    (:CastFailed
      (Development|PrintString "n era p acontecer isso aq n.."))))

(event Custom|Finished
  (Variables|Default|SetisDone true)
  (Rendering|Material|SetMaterial (Variables|Default|GetSphere) 0 "/Game/Puzzles/Materials/DoneMaterial.DoneMaterial")
  (Default|Open (Variables|Default|GetpuzzleDoor)))

(fn ConstructionScript
  (if (Variables|Default|GetisDone)
    (Rendering|Material|SetMaterial (Variables|Default|GetSphere) 0 "/Game/Puzzles/Materials/DoneMaterial.DoneMaterial")))